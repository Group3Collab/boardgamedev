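; Ball actor for what appears to be a Pong-style game, moved by physics velocity on its static mesh.
; BeginPlay launches it along +Y, and actor overlaps are sorted by casts.
; Paddle_Player passes its X velocity to the ball and slightly decrements Y rather than negating it.
; BP_Boundary reapplies velocity unchanged (X times one), while BP_Goal moves the ball to a fixed location without resetting velocity.
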(event EventBeginPlay
  ;[1 1 1] Moving Forward
  (Physics|SetPhysicsLinearVelocity (Variables|Default|GetStaticMesh) "0,500.000000, 0" false "None"))

(event Collision|EventActorBeginOverlap
  (params (OtherActor :type Actor%20Object%20Reference))
  ;[1 1 1] Colllision overlap
  (bind _aspaddle_player (Utilities|Casting|CastToPaddle_Player OtherActor)
    (:then
      (bind _returnvalue (Physics|GetPhysicsLinearVelocity (Variables|/Game/Nick/BluePrints/Paddle_Player.Paddle_Player_C|GetPaddle _aspaddle_player) "None"))
      (bind _returnvalue_2 (Physics|GetPhysicsLinearVelocity (Variables|Default|GetStaticMesh) "None"))
      (Physics|SetPhysicsLinearVelocity (Variables|Default|GetStaticMesh) (Math|Vector|MakeVector (.X (Math|Vector|BreakVector _returnvalue)) (- (.Y (Math|Vector|BreakVector _returnvalue_2)) 1.0) (.Z (Math|Vector|BreakVector _returnvalue_2))) false "None"))
    (:CastFailed
      (Utilities|Casting|CastToBP_Boundary OtherActor
        (:then
          (bind _returnvalue_3 (Physics|GetPhysicsLinearVelocity (Variables|Default|GetStaticMesh) "None"))
          (Physics|SetPhysicsLinearVelocity (Variables|Default|GetStaticMesh) (Math|Vector|MakeVector (* (.X (Math|Vector|BreakVector _returnvalue_3)) 1.0) (.Y (Math|Vector|BreakVector _returnvalue_3)) (.Z (Math|Vector|BreakVector _returnvalue_3))) false "None"))
        (:CastFailed
          (Utilities|Casting|CastToBP_Goal OtherActor)
          (Transformation|SetActorLocation "-440.000000,-70.000000,210.000000" false false))))))

(fn ConstructionScript)